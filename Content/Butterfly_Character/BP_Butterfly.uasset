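; Butterfly actor that starts a wandering flight loop when the player overlaps its Box.
; FindNextLocation randomizes the Sphere's yaw spin, applied on Tick, picks one of six arrow positions, calls StartFlying and repeats after a random delay.
; Start_Flying re-triggers itself by timer, lerping the Sphere a small fixed fraction per step toward the first Arrow; the randomly picked LocationToMove is never read.
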(event OnComponentBeginOverlap(Box)
  (params (OverlappedComponent :type Primitive%20Component%20Object%20Reference) (OtherActor :type Actor%20Object%20Reference) (OtherComp :type Primitive%20Component%20Object%20Reference) (OtherBodyIndex :type Integer) (bFromSweep :type Boolean) (SweepResult :type Hit%20Result%20Structure%20%28by%20ref%29))
  ;[1 1 1] Collision
  (if (== OtherActor (Game|GetPlayerCharacter 0))
    (CallFunction|FindNextLocation)))

(event Custom|Start_Flying
  (bind _sphere (Variables|Default|GetSphere))
  ;[1 1 1] Butterfly starts moving to arrows locations "Start_Flying" Event
  (Variables|Default|SetAlpha 0.0)
  (Utilities|Time|SetTimerbyEvent (delegate Custom|Start_Flying) 0.2)
  (Variables|Default|SetAlpha (+ (Variables|Default|GetAlpha) 0.05))
  (Transformation|SetWorldLocation _sphere (Math|Vector|Lerp(Vector) (Transformation|GetWorldLocation _sphere) (Transformation|GetWorldLocation (Variables|Default|GetArrow)) (Variables|Default|GetAlpha)) false false))

(event Custom|FindNextLocation
  (bind _arrow (Variables|Default|GetArrow))
  (bind _arrow2 (Variables|Default|GetArrow2))
  (bind _arrow3 (Variables|Default|GetArrow3))
  (bind _arrow4 (Variables|Default|GetArrow4))
  (bind _arrow5 (Variables|Default|GetArrow5))
  (bind _arrow1 (Variables|Default|GetArrow1))
  (bind _array (Utilities|Array|MakeArray _arrow _arrow1 _arrow2 _arrow3 _arrow4 _arrow5))
  ;[1 1 1] Bounce between arrow locations randomly
  (Variables|Default|SetDelta%20Rotation%20Z%20%28Yaw%29 (Math|Random|RandomFloatinRange -5.0 5.0))
  (Variables|Default|SetLocationToMove (Transformation|GetWorldLocation (Utilities|Array|Get(acopy) _array (Math|Random|RandomIntegerinRange 0 (Utilities|Array|LastIndex _array)))))
  (CallFunction|StartFlying)
  (Utilities|FlowControl|Delay (Math|Random|RandomFloatinRange 1.5 2.5))
  (CallFunction|FindNextLocation))

(event EventBeginPlay)

(event EventTick
  (params (DeltaSeconds :type Float%20%28single-precision%29))
  (Transformation|AddLocalRotation (Variables|Default|GetSphere) (Math|Rotator|MakeRotator 0.0 0.0 (Variables|Default|GetDelta%20Rotation%20Z%20%28Yaw%29)) false false))

(fn ConstructionScript)