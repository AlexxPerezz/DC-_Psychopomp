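; Guide butterfly that flies a spline path out of the cave once the player enters its Box trigger.
; A timeline scaled by TimeToCompleteSeconds moves and rotates the actor along the first BP_SplinePath found.
; The player leaving the Box reloads the current level after a short delay, serving as game over.
; Random arrow hopping and question-location AI movement have no entry point from the overlap flow; BeginPath is marked as graveyard.
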(event OnComponentEndOverlap(Box)
  (params (OverlappedComponent :type Primitive%20Component%20Object%20Reference) (OtherActor :type Actor%20Object%20Reference) (OtherComp :type Primitive%20Component%20Object%20Reference) (OtherBodyIndex :type Integer))
  ;[1 1 1] When player leaves box collision > Start Game Over (Respawn at Begining)
  (if (== OtherActor (Game|GetPlayerCharacter 0))
    (Utilities|FlowControl|Delay 0.2)
    (bind _returnvalue (Game|GetCurrentLevelName true))
    (Game|OpenLevel(byName) (Utilities|String|StringToName _returnvalue))))

(event OnComponentBeginOverlap(Box)
  (params (OverlappedComponent :type Primitive%20Component%20Object%20Reference) (OtherActor :type Actor%20Object%20Reference) (OtherComp :type Primitive%20Component%20Object%20Reference) (OtherBodyIndex :type Integer) (bFromSweep :type Boolean) (SweepResult :type Hit%20Result%20Structure%20%28by%20ref%29))
  ;[1 1 1] Collision - When player enters > Butterfly will begin flying its path out of the cave
  (if (== OtherActor (Game|GetPlayerCharacter 0))
    (Utilities|FlowControl|Delay 0.2)
    (bind _returnvalue (Actor|GetActorOfClass "/Game/Butterfly_Character/BP_SplinePath.BP_SplinePath_C"))
    (Variables|Default|SetSplineREF _returnvalue)
    (CallFunction|MoveButterfly)))

(event Custom|MoveButterfly
  (bind _splineref (Variables|Default|GetSplineREF))
  (bind _spline (Variables|/Game/Butterfly_Character/BP_SplinePath.BP_SplinePath_C|GetSpline _splineref))
  (Components|Timeline|SetPlayRate (Variables|Default|GetMoveButterfly_T) (/ 1.0 (Variables|Default|GetTimeToComplete%28Seconds%29)))
  (bind _newtrack_0 (Timeline|MoveButterfly_T Play)
    (:Update
      (Transformation|SetActorTransform (Math|Transform|MakeTransform (Spline|GetLocationatDistanceAlongSpline _spline (Math|Float|Lerp 0.0 (Spline|GetSplineLength (Variables|/Game/Butterfly_Character/BP_SplinePath.BP_SplinePath_C|GetSpline (Variables|Default|GetSplineREF))) _newtrack_0) "World") (Spline|GetRotationatDistanceAlongSpline _spline (Math|Float|Lerp 0.0 (Spline|GetSplineLength (Variables|/Game/Butterfly_Character/BP_SplinePath.BP_SplinePath_C|GetSpline (Variables|Default|GetSplineREF))) _newtrack_0) "Local") "1,1,1")))))

(event Custom|BeginPath
  ;[1 1 1] Graveyard IGNORE
  (if (Variables|Path|GetQuestion%20Location%201)
    (Utilities|QuestionLocations false false false false
      (:Out
        (AI|AIMoveTo (Variables|Actor|GetSphere) 0 (Variables|Path|GetLocation%201) 0 5.0 false)))))

(event Custom|FindNextLocation
  (bind _arrow (Variables|Default|GetArrow))
  (bind _arrow1 (Variables|Default|GetArrow1))
  (bind _arrow2 (Variables|Default|GetArrow2))
  (bind _arrow3 (Variables|Default|GetArrow3))
  (bind _arrow4 (Variables|Default|GetArrow4))
  (bind _arrow5 (Variables|Default|GetArrow5))
  (bind _array (Utilities|Array|MakeArray _arrow _arrow1 _arrow2 _arrow3 _arrow4 _arrow5))
  ;[1 1 1] Bounce between arrow locations randomly
  (Variables|Default|SetLocationToMove (Transformation|GetWorldLocation (Utilities|Array|Get(acopy) _array (Math|Random|RandomIntegerinRange 0 (Utilities|Array|LastIndex _array)))))
  (CallFunction|StartFlying)
  (Utilities|FlowControl|Delay (Math|Random|RandomFloatinRange 1.5 2.5))
  (CallFunction|FindNextLocation))

(event Custom|Start_Flying
  (bind _sphere (Variables|Actor|GetSphere))
  ;[1 1 1] "Start_Flying" Event - Butterfly starts moving to arrows locations
  (Variables|Components|SetAlpha 0.0)
  (Utilities|Time|SetTimerbyEvent (delegate Custom|Start_Flying) 0.2)
  (Variables|Components|SetAlpha (+ (Variables|Components|GetAlpha) 0.01))
  (Transformation|SetWorldLocation _sphere (Math|Vector|Lerp(Vector) (Transformation|GetWorldLocation _sphere) (Transformation|GetWorldLocation (Variables|Default|GetArrow)) (Variables|Components|GetAlpha)) false false))

(event EventBeginPlay)

(event EventTick
  (params (DeltaSeconds :type Float%20%28single-precision%29)))

(fn ConstructionScript)