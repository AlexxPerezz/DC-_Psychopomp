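; AC_Dialogue_Component is an actor component on both player and NPC that runs branching, data-table-driven dialogue.
; The NPC's component requests dialogue, and the player's accepts or denies it, then creates the NPC's chosen widget and talks to it through BPI_Dialogue.
; Each line row drives sound, animations, choices, table swaps and condition branches.
; Participant events and condition checks fire by function name via timers, with completion and results reported back.
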(event Custom|Send_Widget_Navigation_Request
  (params (Navigation_Type :type E_UI_Navigation_Request_Type%20Enum :default "NewEnumerator0"))
  ;[1 1 1] Alternative Navigation
  ;;[1 1 1] There may be circumstances where you want to navigate the dialogue widget without a mouse, ex. Gamepad.
  ;;
  ;; If so you can send this message from the player Character on a gamepad input to send a navigation request to the widget.
  (Class|BPIDialogue|SendUINavigationRequest(Message) (Variables|DoNotTouch|GetDialogue_Widget_Ref) Navigation_Type))

(event Custom|Fire_Event_In_Dialogue_Participant
  (params (Event%20Name :type Name))
  ;[1 1 1] Fire events to dialogue participant
  (Utilities|Time|SetTimerbyFunctionName (Variables|DoNotTouch|GetDialogue_Participant_Actor) (Utilities|String|ToString(Name) Event%20Name) 0.1))

(event Custom|Handle_Dialogue_Request
  (params (Initiating_Participant :type Actor%20Object%20Reference))
  ;[1 1 1] Player Character responds to the NPCs request for dialogue
  ;;[1 1 1] From the Player Character "AC_Dialogue_Component" actor component, the Handle_Dialogue_Request function is called.
  ;;
  ;; From the Player Characters "AC_Dialogue_Component" we re-verify the NPCs "AC_Dialogue_Component" also check if the Player characters "Can_Enter_Dialogue" boolean inside the Player Characters "AC_Dialogue_Component" is set to true.
  ;;
  ;; If the "AC_Dialogue_Component" inside the NPC or Dialogue Participant is found, And the Player characters "Can_Enter_Dialogue" boolean inside the Player Characters "AC_Dialogue_Component" is set to true, we move on to the next step.
  (bind (_actor_checked _dialogue_component_found) (Utilities|HasDialogueComponent Initiating_Participant)
    (:Dialogue_Component_Valid
      (if (Variables|Options_For_Player|GetCan_Enter_Dialogue)
        ;;[1 1 1] Set the Dialogue Participant Actor reference to the actor that has been checked out by the macro, and Set the DP Dialogue Component the that NPCs "AC_Dialogue_Component".
        (Variables|DoNotTouch|SetDialogue_Participant_Actor _actor_checked)
        (Variables|DoNotTouch|SetDP_Dialogue_Component _dialogue_component_found)
        ;;[1 1 1] We re-verify that the Player Character Implements the "AC_Dialogue_Component" actor component. If True, Set the Player Character Actor reference to the actor that has been checked out by the macro, and Set the PC Dialogue Component the that Players "AC_Dialogue_Component".
        (bind (_actor_checked_2 _dialogue_component_found_2) (Utilities|HasDialogueComponent (Components|GetOwner))
          (:Dialogue_Component_Valid
            (Variables|DoNotTouch|SetPlayer_Character_Actor _actor_checked_2)
            (Variables|DoNotTouch|SetPC_Dialogue_Component _dialogue_component_found_2)
            ;;[1 1 1] If everything checks out, we fire the Accept Dialogue Request function from the Player Characters "AC_Dialogue_Component" to the NPCs "AC_Dialogue_Component"
            (Utilities|FlowControl|Sequence
              (:then_0
                ;[1 1 1] Player accepts NPCs dialogue request
                ;;[1 1 1] If everything checks out, the Player Characters "AC_Dialogue_Component" accepts the dialogue request. We only want this function to fire once until our next interaction to keep spamming interact from firing this multiple times and creating more widgets in memory.
                (Utilities|FlowControl|DoOnce false) ; enters at Reset
              )
              (:then_1
                (CallFunction|AcceptDialogueRequest))))
          (:Dialogue_Component_Not_Valid
            ;;[1 1 1] If we could not find the "AC_Dialogue_Component" in the NPC, or our Player characters "Can_Enter_Dialogue" boolean inside the Player Characters "AC_Dialogue_Component" is set to false, we deny the dialogue request inside the NPCs "AC_Dialogue_Component" and go no further.
            (CallFunction|DenyDialogueRequest _dialogue_component_found :!label _label)))
        (else
          (goto _label))))
    (:Dialogue_Component_Not_Valid
      (goto _label))))

(event Custom|Deny_Dialogue_Request
  ;[1 1 1] Dialogue request denied by player
  ;;[1 1 1] In the NPCs "AC_Dialogue_Component" we set its Attempting_Dialogue_With_Player value back to false if we recieve the Deny_Dialogue_Request function call.
  (Variables|DoNotTouch|SetAttempting_Dialogue_With_Player? false))

(event Custom|Accept_Dialogue_Request
  (bind _dp_dialogue_component (Variables|DoNotTouch|GetDP_Dialogue_Component))
  ;[1 1 1] Player accepts NPCs dialogue request
  ;;[1 1 1] If everything checks out, the Player Characters "AC_Dialogue_Component" accepts the dialogue request. We only want this function to fire once until our next interaction to keep spamming interact from firing this multiple times and creating more widgets in memory.
  (Utilities|FlowControl|DoOnce false
    (:Completed
      ;;[1 1 1] Send a message to player and participant to let them know dialogue has began.
      (Class|BPIDialogue|ActivateDialogue(Message) (Variables|DoNotTouch|GetPlayer_Character_Actor))
      (Class|BPIDialogue|ActivateDialogue(Message) (Variables|DoNotTouch|GetDialogue_Participant_Actor))
      ;;[1 1 1] We Create the Widget found in the NPCs "Desired_Dialogue_Widget" class reference, and ask if it implements the "BPI_Dialogue" interface. If not, we break out of dialogue to prevent softlock. If so, We set the Dialogue Widget Reference to the newly created widget and move on.
      (bind _returnvalue (UserInterface|CreateWidget (Variables|AC_Dialogue_Component_C|GetDesired_Dialogue_Widget (Variables|DoNotTouch|GetDP_Dialogue_Component)) (Game|GetPlayerController 0)))
      (if (Utilities|DoesObjectImplementInterface _returnvalue "/Game/Dynamic_Dialogue_System/Blueprints/Interfaces/BPI_Dialogue.BPI_Dialogue_C")
        (Variables|DoNotTouch|SetDialogue_Widget_Ref _returnvalue)
        ;;[1 1 1] We set the Can_Dialogue_Advance? and Dialogue_Widget_Open? variables to false by default to be controlled later.
        (Variables|DoNotTouch|SetCan_Dialogue_Advance? false)
        (Variables|DoNotTouch|SetDialogue_Widget_Open? false)
        ;;[1 1 1] We grab the NPC or Dialogue Participants "AC_Dialogue_Component" and find its Dialogue_Entrance_ID, and its Dialogue_Participant_Data_Table variables, and set our Buffered_Entrance_ID, and Buffered_Data_Table variables respectfully in the Player Characters "AC_Dialogue_Component". Then we forward our component to the newly created Dialogue Widget Ref.
        (Variables|AC_Dialogue_Component_C|SetBuffered_Entrance_ID _dp_dialogue_component (Variables|AC_Dialogue_Component_C|GetDialogue_Entrance_ID _dp_dialogue_component))
        (Variables|AC_Dialogue_Component_C|SetBuffered_Data_Table _dp_dialogue_component (Variables|AC_Dialogue_Component_C|GetDialogue_Participant_Data_Table _dp_dialogue_component))
        (Class|BPIDialogue|ForwardDialogueComponent(Message) (Variables|DoNotTouch|GetDialogue_Widget_Ref) self)
        ;;[1 1 1] We Start the dialogue line.
        (CallFunction|BeginDialogueLine)
        (else
          (Variables|DoNotTouch|SetDialogue_Widget_Ref _returnvalue)
          (CallFunction|DisengageDialogue))))))

(event Custom|Instigate_Advance_Dialogue
  ;[1 1 1] Advance dialogue
  ;;[1 1 1] Instigate_Advance_Dialogue is fired from the Player Characters blueprint based on an imput you select.
  ;;
  ;; We ask the Players "AC_Dialogue_Component" if Can_Dialogue_Advance? is set to True.
  ;; If False, we do nothing, as this should not affect the dialogue.
  ;; If True, we ask if this is the Last_Line_in_Dialogue?.
  ;;
  ;; If True, we disengage the dialogue since it is completed.
  ;; If False, We attempt to find the next dialogue line with the Decide_Next_Dialogue_Line function, and Set the Can_Dialogue_Advance? to false.
  (if (Variables|DoNotTouch|GetCan_Dialogue_Advance?)
    (if (Utilities|Struct|BreakF_Dialogue_Entry_Info (Variables|DoNotTouch|GetDialogue_Entry_Info))
      (CallFunction|DisengageDialogue)
      (else
        (CallFunction|DecideNextDialogueLine)
        (Variables|DoNotTouch|SetCan_Dialogue_Advance? false)))
    (else
      (Class|BPIDialogue|SignalAdvanceAttempted(Message) (Variables|DoNotTouch|GetDialogue_Widget_Ref)))))

(event Custom|Complete_Line
  (bind _dialogue_entry_info (Variables|DoNotTouch|GetDialogue_Entry_Info))
  (bind (_line_lead_to_choice_ _dialogue_choices) (Utilities|Struct|BreakF_Dialogue_Entry_Info _dialogue_entry_info))
  ;[1 1 1] Complete the line
  ;;[1 1 1] After events, Animations, and sound have been fired, we  check if the line should end with options. If so we set Can_Dialogue_Advance? to false.
  ;;
  ;; If Show_Mouse_when_Dialogue_Options_Open? is true, we fire the function to show the mouse cursor, then send a message to the Dialogue Widget to Open Options. If Show_Mouse_when_Dialogue_Options_Open? is false we just send a message to the Dialogue Widget to Open Options
  (if _line_lead_to_choice_
    (Variables|DoNotTouch|SetCan_Dialogue_Advance? false)
    (if (Variables|Options_For_Player|GetShow_Mouse_When_Dialogue_Options_Open?)
      (CallFunction|ShowPlayerMouse true))
    (Class|BPIDialogue|WidgetOpenDialogueOptions(Message) (Variables|DoNotTouch|GetDialogue_Widget_Ref) _dialogue_choices)))

(event Custom|Confirm_Event_Finished
  (bind _dialogue_entry_info (Variables|DoNotTouch|GetDialogue_Entry_Info))
  (bind _dialogue_widget_ref (Variables|DoNotTouch|GetDialogue_Widget_Ref))
  (bind (_participant_icon _player_icon _trigger_event_ _trigger_event_time _trigger_event_name _wait_for_event_to_finish_ _delay_show_dialogue_bubble) (Utilities|Struct|BreakF_Dialogue_Entry_Info _dialogue_entry_info))
  (bind _returnvalue (> _delay_show_dialogue_bubble 0.0))
  ;[1 1 1] Handle initial event firing on the line id executing.
  ;;[1 1 1] If the event to fire is complete, continue on in the dialocue.
  (Utilities|FlowControl|DoOnce false
    (:Completed
      ;;[1 1 1] Decide if the widget is already open, if not, should it delay opening
      (if (Variables|DoNotTouch|GetDialogue_Widget_Open?)
        ;;[1 1 1] If the dialogue widget is hidden, Unhide the widget.
        (if _returnvalue
          (Utilities|FlowControl|Delay _delay_show_dialogue_bubble))
        (Class|BPIDialogue|DisplayDialogueWidget(Message) (Variables|DoNotTouch|GetDialogue_Widget_Ref))
        (CallFunction|PlayAnimationandSound)
        (CallFunction|CompleteLine)
        (Variables|DoNotTouch|SetDialogue_Widget_Open? true)
        (else
          (if _returnvalue
            (Utilities|FlowControl|Delay _delay_show_dialogue_bubble))
          ;;[1 1 1] If this is the first time opening the dialogue widget, add the widget to the viewport.
          (UserInterface|Viewport|AddtoViewport _dialogue_widget_ref 1)
          (Input|SetInputModeGameandUI (Game|GetPlayerController 0) _dialogue_widget_ref "LockAlways" true)
          (Class|BPIDialogue|DisplayDialogueWidget(Message) (Variables|DoNotTouch|GetDialogue_Widget_Ref))
          (Variables|DoNotTouch|SetDialogue_Widget_Open? true)
          (CallFunction|PlayAnimationandSound)
          (CallFunction|CompleteLine))))))

(event Custom|Begin_Dialogue_Line
  (bind _dialogue_entry_info (Variables|DoNotTouch|GetDialogue_Entry_Info))
  (bind _dialogue_widget_ref (Variables|DoNotTouch|GetDialogue_Widget_Ref))
  (bind _dp_dialogue_component (Variables|DoNotTouch|GetDP_Dialogue_Component))
  (bind _dialogue_entry_info_2 (Variables|DoNotTouch|GetDialogue_Entry_Info))
  (bind (_participant_icon _player_icon _trigger_event_ _trigger_event_time _trigger_event_name _wait_for_event_to_finish_ _delay_show_dialogue_bubble) (Utilities|Struct|BreakF_Dialogue_Entry_Info _dialogue_entry_info))
  (bind (_participant_icon_2 _player_icon_2 _changes_dialogue_entrance_id_ _entrance_id_to_swap_to _changes_dialogue_entrance_data_table _entrance_dialogue_table_changed_to) (Utilities|Struct|BreakF_Dialogue_Entry_Info _dialogue_entry_info_2))
  (bind _returnvalue (> _delay_show_dialogue_bubble 0.0))
  ;[1 1 1] Find and buffer the dialogue line info from the data table, at the entry ID listed from the Dialogue Participant. If a row is found,we move on.
  ;;[1 1 1] On the Begin_Dialogue_Line function call, we set the Can_Dialogue_Advance? variable to False so advancement can be controlled through your desired Dialogue Widget.
  ;;
  ;; We set Buffer_Event_To_Fire? to Fase so it can be decided in further script in case an event was buffered to fire in the last line.
  ;;
  ;; We validate that the Buffered_Entrance_ID exists in the Buffered_Data_Table reference. If the Buffered_Entrance_ID exists in the Buffered_Data_Table we move on. If not, we break out of the dialogue to prevent softlock.
  (Variables|DoNotTouch|SetCan_Dialogue_Advance? false)
  (Variables|DoNotTouch|SetBuffer_Event_To_Fire? false)
  (Utilities|ValidateDialogueEntryLine (Variables|AC_Dialogue_Component_C|GetBuffered_Data_Table _dp_dialogue_component) (Variables|AC_Dialogue_Component_C|GetBuffered_Entrance_ID _dp_dialogue_component)
    (:Line_Found
      ;[1 1 1] If the dialogue entry requested is not valid, break the dialogue cycle to prevent softlock
      ;;[1 1 1] If we want the current line to permanently swap the NPCs Entrance_ID based on the Dialogue_Entry_info, we do that right now.
      (if _changes_dialogue_entrance_id_
        (Variables|AC_Dialogue_Component_C|SetDialogue_Entrance_ID (Variables|DoNotTouch|GetDP_Dialogue_Component) _entrance_id_to_swap_to))
      ;;[1 1 1] If we want the current line to permanently swap the NPCs Dialogue_Participant_Data_Table based on the Dialogue_Entry_info, we do that right now.
      (if _changes_dialogue_entrance_data_table
        (Variables|AC_Dialogue_Component_C|SetDialogue_Participant_Data_Table (Variables|DoNotTouch|GetDP_Dialogue_Component) _entrance_dialogue_table_changed_to))
      ;;[1 1 1] If the Dialogue_Entry_Found variable (Which was set in our "Validate_Dialogue_Entry_Line" Macro) is set to False, a line was not found and we disengage the dialogue to prevent softlock. If it was found, we forward our dialogue component to the desired Dialogue Widget Reference and move on.
      (if (Variables|DoNotTouch|GetDialogue_Entry_Found) ; Check if a dialogue entry was found.\nIf not something has been broken in\nthe references, and we should exit the\ndialogue.
        (Class|BPIDialogue|ForwardDialogueComponent(Message) (Variables|DoNotTouch|GetDialogue_Widget_Ref) (Variables|DoNotTouch|GetPC_Dialogue_Component))
        ;[1 1 1] Handle initial event firing on the line id executing.
        (Utilities|FlowControl|Sequence
          (:then_0
            ;;[1 1 1] If the line should trigger an event, determine if the event should be before or after.
            (if _trigger_event_
              (switch Utilities|FlowControl|Switch|SwitchonE_Event_Fire_Timing_Type _trigger_event_time
                (:NewEnumerator0
                  ;;[1 1 1] Fire an event to the dialogue participant.
                  (CallFunction|FireEventinDialogueParticipant _trigger_event_name)
                  (if (not _wait_for_event_to_finish_)
                    ;;[1 1 1] Decide if the widget is already open, if not, should it delay opening
                    (if (Variables|DoNotTouch|GetDialogue_Widget_Open?) :!label _label
                      ;;[1 1 1] If the dialogue widget is hidden, Unhide the widget.
                      (if _returnvalue
                        (Utilities|FlowControl|Delay _delay_show_dialogue_bubble))
                      (Class|BPIDialogue|DisplayDialogueWidget(Message) (Variables|DoNotTouch|GetDialogue_Widget_Ref))
                      (CallFunction|PlayAnimationandSound)
                      (CallFunction|CompleteLine)
                      (Variables|DoNotTouch|SetDialogue_Widget_Open? true)
                      (else
                        (if _returnvalue
                          (Utilities|FlowControl|Delay _delay_show_dialogue_bubble))
                        ;;[1 1 1] If this is the first time opening the dialogue widget, add the widget to the viewport.
                        (UserInterface|Viewport|AddtoViewport _dialogue_widget_ref 1)
                        (Input|SetInputModeGameandUI (Game|GetPlayerController 0) _dialogue_widget_ref "LockAlways" true)
                        (Class|BPIDialogue|DisplayDialogueWidget(Message) (Variables|DoNotTouch|GetDialogue_Widget_Ref))
                        (Variables|DoNotTouch|SetDialogue_Widget_Open? true)
                        (CallFunction|PlayAnimationandSound)
                        (CallFunction|CompleteLine)))))
                (:NewEnumerator1
                  ;;[1 1 1] If the event happens after, create a buffer for the event to fire at the end of the line.
                  (Variables|DoNotTouch|SetBuffered_Event_To_Fire_Name _trigger_event_name)
                  (Variables|DoNotTouch|SetBuffer_Event_To_Fire? true)
                  (goto _label)))
              (else
                (goto _label))))
          (:then_1
            ;;[1 1 1] If the event to fire is complete, continue on in the dialocue.
            (Utilities|FlowControl|DoOnce false) ; enters at Reset
          ))
        (else
          (CallFunction|DisengageDialogue))))
    (:Line_Not_Found
      (CallFunction|DisengageDialogue))))

(event Custom|Play_Animation_And_Sound
  (bind _dialogue_entry_info (Variables|DoNotTouch|GetDialogue_Entry_Info))
  (bind (_play_sound_ _sound_to_play _dialogue_participant_plays_animation_ _dialogue_participant_animation_to_play _player_plays_animation_ _player_animation_to_play _audio_delay_tweak _participant_animation_delay_tweak _character_animation_delay_tweak) (Utilities|Struct|BreakF_Dialogue_Entry_Info _dialogue_entry_info))
  ;[1 1 1] Play animations and sound
  (Utilities|FlowControl|Sequence
    (:then_0
      (if _play_sound_
        (if (> _audio_delay_tweak 0.0)
          (Utilities|FlowControl|Delay _audio_delay_tweak))
        (CallFunction|SpawnGlobalSoundEffect _sound_to_play)))
    (:then_1
      (if _dialogue_participant_plays_animation_
        (if (> _participant_animation_delay_tweak 0.0)
          (Utilities|FlowControl|Delay _participant_animation_delay_tweak))
        (Class|BPIDialogue|SkeletalMeshPlayAnimation(Message) (Variables|DoNotTouch|GetDialogue_Participant_Actor) _dialogue_participant_animation_to_play)))
    (:then_2
      (if _player_plays_animation_
        (if (> _character_animation_delay_tweak 0.0)
          (Utilities|FlowControl|Delay _character_animation_delay_tweak))
        (Class|BPIDialogue|SkeletalMeshPlayAnimation(Message) (Variables|DoNotTouch|GetPlayer_Character_Actor) _player_animation_to_play)))))

(event Custom|Decide_Next_Dialogue_Line
  (bind _dp_dialogue_component (Variables|DoNotTouch|GetDP_Dialogue_Component))
  (bind _dialogue_entry_info (Variables|DoNotTouch|GetDialogue_Entry_Info))
  (bind _dialogue_entry_info_2 (Variables|DoNotTouch|GetDialogue_Entry_Info))
  (bind (_dialogue_line_requires_condition_ _dialogue_condition_check_function_name) (Utilities|Struct|BreakF_Dialogue_Entry_Info _dialogue_entry_info_2))
  (bind (_this_line_swaps_data_tables_ _data_table_to_swap_to) (Utilities|Struct|BreakF_Dialogue_Entry_Info _dialogue_entry_info))
  ;[1 1 1] Advance dialogue
  ;;[1 1 1] The Decide_Next_Dialogue_Line function Asks if the current dialogue line should swap the Buffered_Data_Table.
  ;; If False, We Move on.
  ;; If True, We swap the Buffered_Data_Table to the data table coming in from the Data_Table_to_Swap_To variable in the dialogue line.
  ;;
  ;; We then set the Buffered_Entrance_ID to the Lead_to_ID variable in the dialogue line.
  ;;
  ;; Then we ask if the current configuration of Entrance ID and Data table are valid.
  ;; If not valid, Something has gone wrong and we Disengage the Dialogue.
  ;; If so, we move on
  (if _this_line_swaps_data_tables_
    (Variables|AC_Dialogue_Component_C|SetBuffered_Data_Table (Variables|DoNotTouch|GetDP_Dialogue_Component) _data_table_to_swap_to))
  (bind _output_get (Variables|AC_Dialogue_Component_C|SetBuffered_Entrance_ID _dp_dialogue_component (Utilities|Struct|BreakF_Dialogue_Entry_Info (Variables|DoNotTouch|GetDialogue_Entry_Info))))
  (Utilities|ValidateDialogueEntryLine (Variables|AC_Dialogue_Component_C|GetBuffered_Data_Table _dp_dialogue_component) _output_get
    (:Line_Found
      ;;[1 1 1] Ask if the next line requires a condition. If so, fire an event to the dialogue participant to resolve the condition.
      (if _dialogue_line_requires_condition_
        (CallFunction|FireEventinDialogueParticipant _dialogue_condition_check_function_name)
        (else
          ;;[1 1 1] If no condition is needed fire Advance Dialogue message to the widget.
          (if (Variables|DoNotTouch|GetDialogue_Entry_Found)
            (if (Variables|Options_For_Player|GetShow_Mouse_When_Dialogue_Options_Open?)
              (CallFunction|ShowPlayerMouse false))
            (Class|BPIDialogue|AdvanceDialogue(Message) (Variables|DoNotTouch|GetDialogue_Widget_Ref) (Variables|DoNotTouch|GetDialogue_Entry_Info))))))
    (:Line_Not_Found
      (CallFunction|DisengageDialogue))))

(event Custom|Confirm_Next_Dialogue_Line
  (bind _dp_dialogue_component (Variables|DoNotTouch|GetDP_Dialogue_Component))
  (bind _dialogue_entry_info (Variables|DoNotTouch|GetDialogue_Entry_Info))
  (bind (_condition_check_failed_lead_to_id _condition_failed_lead_to_data_table) (Utilities|Struct|BreakF_Dialogue_Entry_Info _dialogue_entry_info))
  ;[1 1 1] Advance dialogue
  ;;[1 1 1] If the dialogue condition check fails, we verify the line id and advance down the condition check failed tree.
  (Variables|AC_Dialogue_Component_C|SetBuffered_Data_Table (Variables|DoNotTouch|GetDP_Dialogue_Component) _condition_failed_lead_to_data_table)
  (bind _output_get (Variables|AC_Dialogue_Component_C|SetBuffered_Entrance_ID _dp_dialogue_component _condition_check_failed_lead_to_id))
  (Utilities|ValidateDialogueEntryLine (Variables|AC_Dialogue_Component_C|GetBuffered_Data_Table _dp_dialogue_component) _output_get
    (:Line_Found
      (if (Variables|Options_For_Player|GetShow_Mouse_When_Dialogue_Options_Open?)
        (CallFunction|ShowPlayerMouse false))
      (Class|BPIDialogue|AdvanceDialogue(Message) (Variables|DoNotTouch|GetDialogue_Widget_Ref) (Variables|DoNotTouch|GetDialogue_Entry_Info)))
    (:Line_Not_Found
      (CallFunction|DisengageDialogue))))

(event Custom|Request_Dialogue
  (params (Player :type Actor%20Object%20Reference))
  ;[1 1 1] NPC Fires request to initiate dialogue with player character
  ;;[1 1 1] Request_Dialogue is an event fired from the NPC or Dialogue Participants blueprint.
  ;;
  ;; We verify that both NPC & Player Character implement the "AC_Dialogue_Component" actor component.
  ;; Then we set the reference to the Player Characters "AC_Dialogue_Component" and fire the "Handle_Dialogue_Request" function to it.
  (Variables|DoNotTouch|SetAttempting_Dialogue_With_Player? true)
  (bind _actor_checked (Utilities|HasDialogueComponent (Components|GetOwner))
    (:Dialogue_Component_Valid
      (bind (_actor_checked_2 _dialogue_component_found) (Utilities|HasDialogueComponent Player)
        (:Dialogue_Component_Valid
          (Variables|DoNotTouch|SetPlayer_Character_Actor _actor_checked_2)
          (bind _output_get (Variables|DoNotTouch|SetPC_Dialogue_Component _dialogue_component_found))
          (CallFunction|HandleDialogueRequest _output_get _actor_checked))))))

(event EventBeginPlay)

(event EventTick
  (params (DeltaSeconds :type Float%20%28single-precision%29)))

(event EventComponentSetAdvancePossible
  (params (Advance_Possible_Value :type Boolean))
  ;[1 1 1] Advance dialogue
  ;;[1 1 1] Sets if the player can advance the dialogue.
  (Variables|DoNotTouch|SetCan_Dialogue_Advance? Advance_Possible_Value))

(event EventBeginNewDialogueLine
  ;[1 1 1] Advance dialogue
  ;;[1 1 1] Confirm that a new line should play.
  (CallFunction|BeginDialogueLine))

(event EventConfirmDialogueConditionCheck
  (params (Condition_State :type Boolean))
  ;[1 1 1] Advance dialogue
  ;;[1 1 1] If the condition check returns true, Fire the Advance Dialogue Message to the Dialogue Widget.
  (if Condition_State
    (if (Variables|DoNotTouch|GetDialogue_Entry_Found)
      (if (Variables|Options_For_Player|GetShow_Mouse_When_Dialogue_Options_Open?)
        (CallFunction|ShowPlayerMouse false))
      (Class|BPIDialogue|AdvanceDialogue(Message) (Variables|DoNotTouch|GetDialogue_Widget_Ref) (Variables|DoNotTouch|GetDialogue_Entry_Info)))
    (else
      (CallFunction|ConfirmNextDialogueLine))))

(event EventFiredEventComplete
  ;[1 1 1] Fire events to dialogue participant
  (CallFunction|ConfirmEventFinished))

(event EventDialogueOptionSelected
  (params (Dialogue_Option_Info :type F%20Dialogue%20Response%20Info%20Structure))
  (bind (_option_lead_to_id _should_swap_dialogue_tables _swapped_dialogue_table) (Utilities|Struct|BreakF_Dialogue_Response_Info Dialogue_Option_Info))
  ;[1 1 1] Handle dialogue option selected
  ;;[1 1 1] When we recieve the messge Dialogue_Option_Selected from the Dialogue Widget, We get its lead to ID and set our Buffered ID to that Value.
  ;;
  ;; Next we ask if the data table should swap on this selection. If so we set our Buffered_Dialogue_Table to the Swapped_Dialogue_Table from the Option Button.
  ;;
  ;; And finally we hide the mouse cursor if the  Show_Mouse_when_Dialogue_Options_Open? is set to true.
  (Variables|AC_Dialogue_Component_C|SetBuffered_Entrance_ID (Variables|DoNotTouch|GetDP_Dialogue_Component) _option_lead_to_id)
  (if _should_swap_dialogue_tables
    (Variables|AC_Dialogue_Component_C|SetBuffered_Data_Table (Variables|DoNotTouch|GetDP_Dialogue_Component) _swapped_dialogue_table))
  (if (Variables|Options_For_Player|GetShow_Mouse_When_Dialogue_Options_Open?)
    (CallFunction|ShowPlayerMouse false)))

(fn DisengageDialogue
  (bind _returnvalue (Game|GetPlayerController 0))
  (Class|BPIDialogue|CloseDialogeWidget(Message) (Variables|DoNotTouch|GetDialogue_Widget_Ref))
  (Class|BPIDialogue|DeactivateDialogue(Message) (Variables|DoNotTouch|GetPlayer_Character_Actor))
  (Class|BPIDialogue|DeactivateDialogue(Message) (Variables|DoNotTouch|GetDialogue_Participant_Actor))
  (Variables|DoNotTouch|SetCan_Dialogue_Advance? false)
  (Variables|/Script/Engine.PlayerController|SetbShowMouseCursor _returnvalue false)
  (Input|SetInputModeGameOnly _returnvalue)
  (Variables|DoNotTouch|SetDialogue_Entry_Found false)
  (if (Variables|DoNotTouch|GetBuffer_Event_To_Fire?)
    (CallFunction|FireEventinDialogueParticipant (Variables|DoNotTouch|GetBuffered_Event_To_Fire_Name))))

(fn SpawnGlobalSoundEffect
  (params (Sound_To_Play :type Sound%20Base%20Object%20Reference))
  (bind _returnvalue (Audio|SpawnSound2D Sound_To_Play (Variables|DoNotTouch|GetSound_FX_Multiplier) 1.0 0.0 0))
  (Variables|DoNotTouch|SetCurrent_Sound_Playing _returnvalue))

(fn ShowPlayerMouse
  (params (New_Mouse_Show_State :type Boolean))
  (Variables|/Script/Engine.PlayerController|SetbShowMouseCursor (Game|GetPlayerController 0) New_Mouse_Show_State))