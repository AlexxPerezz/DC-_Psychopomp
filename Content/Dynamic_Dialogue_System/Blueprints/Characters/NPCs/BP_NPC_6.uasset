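; BP_NPC_6 is a demonstration NPC for the dialogue system, showing how dialogue events drive the NPC and the player character.
; Activating dialogue plays a timeline that turns the NPC toward the player, whom it also rotates and stops.
; Deactivating reverses the timeline, re-enables movement and restores the player's camera.
; Separate callable events hand off or restore that camera through the player reference held by the dialogue component.
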(event Custom|Change_Player_Camera
  ;[1 1 1] Demonstration of event calling: Change the players Camera.
  (bind _asbp_player_character (Utilities|Casting|CastToBP_Player_Character (Variables|/Game/Dynamic_Dialogue_System/Blueprints/Components/AC_Dialogue_Component.AC_Dialogue_Component_C|GetPlayer_Character_Actor (Variables|Default|GetAC_Dialogue_Component))))
  (Default|HandOffCamera _asbp_player_character))

(event Custom|Restore_Player_Camera
  ;[1 1 1] Demonstration for event calling: Restores the players camera.
  (bind _asbp_player_character (Utilities|Casting|CastToBP_Player_Character (Variables|/Game/Dynamic_Dialogue_System/Blueprints/Components/AC_Dialogue_Component.AC_Dialogue_Component_C|GetPlayer_Character_Actor (Variables|Default|GetAC_Dialogue_Component))))
  (Default|RestoreCamera _asbp_player_character))

(event EventActivateDialogue
  ;[1 1 1] Fired when Activation of Dialogue begins.
  (Variables|Default|SetIs_In_Dialogue? true)
  (Utilities|FlowControl|Sequence
    (:then_0
      ;[1 1 1] Demonstrates rotating to player
      (bind _newtrack_0 (Timeline|Rotate%20to%20player Play)
        (:Update
          (Transformation|SetActorRotation (Math|Rotator|Lerp(Rotator) (Transformation|GetActorRotation) (Math|Rotator|FindLookatRotation (Transformation|GetActorLocation) (Transformation|GetActorLocation (Variables|/Game/Dynamic_Dialogue_System/Blueprints/Components/AC_Dialogue_Component.AC_Dialogue_Component_C|GetPlayer_Character_Actor (Variables|Default|GetAC_Dialogue_Component)))) _newtrack_0 true)))))
    (:then_1
      ;[1 1 1] Stop players movement
      (bind _asbp_player_character (Utilities|Casting|CastToBP_Player_Character (Variables|/Game/Dynamic_Dialogue_System/Blueprints/Components/AC_Dialogue_Component.AC_Dialogue_Component_C|GetPlayer_Character_Actor (Variables|Default|GetAC_Dialogue_Component))))
      (Default|RotatetoDialogueParticipant _asbp_player_character)
      (Default|StopMovement _asbp_player_character))))

(event EventDeactivateDialogue
  ;[1 1 1] Fired when Activation of Dialogue begins.
  (Variables|Default|SetIs_In_Dialogue? false)
  (Utilities|FlowControl|Sequence
    (:then_0
      ;[1 1 1] Demonstrates rotating to player
      (bind _newtrack_0 (Timeline|Rotate%20to%20player Reverse)
        (:Update
          (Transformation|SetActorRotation (Math|Rotator|Lerp(Rotator) (Transformation|GetActorRotation) (Math|Rotator|FindLookatRotation (Transformation|GetActorLocation) (Transformation|GetActorLocation (Variables|/Game/Dynamic_Dialogue_System/Blueprints/Components/AC_Dialogue_Component.AC_Dialogue_Component_C|GetPlayer_Character_Actor (Variables|Default|GetAC_Dialogue_Component)))) _newtrack_0 true)))))
    (:then_1
      ;[1 1 1] Enable players movement.
      (bind _asbp_player_character (Utilities|Casting|CastToBP_Player_Character (Variables|/Game/Dynamic_Dialogue_System/Blueprints/Components/AC_Dialogue_Component.AC_Dialogue_Component_C|GetPlayer_Character_Actor (Variables|Default|GetAC_Dialogue_Component))))
      (Default|EnableMovement _asbp_player_character))
    (:then_2
      ;[1 1 1] Demonstration for event calling: Restores the players camera.
      (bind _asbp_player_character_2 (Utilities|Casting|CastToBP_Player_Character (Variables|/Game/Dynamic_Dialogue_System/Blueprints/Components/AC_Dialogue_Component.AC_Dialogue_Component_C|GetPlayer_Character_Actor (Variables|Default|GetAC_Dialogue_Component))))
      (Default|RestoreCamera _asbp_player_character_2))))

(fn ConstructionScript
  (|CallParentFunction))