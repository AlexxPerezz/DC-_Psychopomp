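; BP_Signpost is an interactable signpost that starts dialogue with the player through its dialogue component.
; Overlapping its interact area registers it as an interactable with BP_Player_Character, and leaving unregisters it and disengages any active dialogue.
; Interaction requests dialogue from the component, guarded by an IsInDialogue flag that the Activate and Deactivate dialogue events also update.
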(event OnComponentBeginOverlap(Interact_Area)
  (params (OverlappedComponent :type Primitive%20Component%20Object%20Reference) (OtherActor :type Actor%20Object%20Reference) (OtherComp :type Primitive%20Component%20Object%20Reference) (OtherBodyIndex :type Integer) (bFromSweep :type Boolean) (SweepResult :type Hit%20Result%20Structure%20%28by%20ref%29))
  (bind _asbp_player_character (Utilities|Casting|CastToBP_Player_Character OtherActor))
  (Class|BPIInteract|RegisterInteractable(Message) _asbp_player_character self))

(event OnComponentEndOverlap(Interact_Area)
  (params (OverlappedComponent :type Primitive%20Component%20Object%20Reference) (OtherActor :type Actor%20Object%20Reference) (OtherComp :type Primitive%20Component%20Object%20Reference) (OtherBodyIndex :type Integer))
  (bind _asbp_player_character (Utilities|Casting|CastToBP_Player_Character OtherActor))
  (Class|BPIInteract|UnregisterInteractable(Message) _asbp_player_character)
  (if (Variables|Default|GetIs_In_Dialogue?)
    (Default|DisengageDialogue (Variables|/Game/Dynamic_Dialogue_System/Blueprints/Components/AC_Dialogue_Component.AC_Dialogue_Component_C|GetPC_Dialogue_Component (Variables|Default|GetAC_Dialogue_Component)))))

(event EventActivateDialogue
  (Variables|Default|SetIs_In_Dialogue? true))

(event EventDeactivateDialogue
  (Variables|Default|SetIs_In_Dialogue? false))

(event EventInteraction
  (params (Instigator :type Actor%20Object%20Reference))
  (if (not (Variables|Default|GetIs_In_Dialogue?))
    (Variables|Default|SetIs_In_Dialogue? true)
    ;[1 1 1] This is the only function you need to fire to engage the player in dialogue.
    ; Just plug in the execute pin, Plug in a pin that references the Player Character,
    ; and set your own "AC_Dialogue_Component" to the target and you are DONE!
    (Default|RequestDialogue (Variables|Default|GetAC_Dialogue_Component) Instigator)))

(fn ConstructionScript)